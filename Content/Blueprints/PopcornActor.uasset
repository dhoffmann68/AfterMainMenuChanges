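; PopcornActor is a damageable actor that rides along a level spline and is destroyed by first-person projectile hits.
; On BeginPlay, if ActiveCart is set, a timeline scaled by Duration and started at CartStartOffset drives its location and rotation along the spline by distance.
; Each projectile overlap subtracts fixed health until it reaches zero.
; Health bar widget creation and straight-line movement logic are present but never run.
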(event Custom|MovingPopcornActor
  (Components|Timeline|SetPlayRate (Variables|Default|GetMoveActor) (/ 1.0 (Variables|Default|GetDuration)))
  (Components|Timeline|SetNewTime (Variables|Default|GetMoveActor) (Variables|Default|GetCart%20Start%20Offset))
  (bind _alpha (Timeline|MoveActor Play)
    (:Update
      (Variables|Default|SetAlpha _alpha)
      (Transformation|SetActorLocationAndRotation (Spline|GetLocationatDistanceAlongSpline (Variables|/Game/Blueprints/LevelSpline.LevelSpline_C|GetSpline (Variables|Default|GetLevelSplineRef)) (Math|Float|Lerp 0.0 (Spline|GetSplineLength (Variables|/Game/Blueprints/LevelSpline.LevelSpline_C|GetSpline (Variables|Default|GetLevelSplineRef))) (Variables|Default|GetAlpha)) "World") (Spline|GetRotationatDistanceAlongSpline (Variables|/Game/Blueprints/LevelSpline.LevelSpline_C|GetSpline (Variables|Default|GetLevelSplineRef)) (Math|Float|Lerp 0.0 (Spline|GetSplineLength (Variables|/Game/Blueprints/LevelSpline.LevelSpline_C|GetSpline (Variables|Default|GetLevelSplineRef))) (Variables|Default|GetAlpha)) "World")))))

(event EventBeginPlay
  (if (Variables|Default|GetActiveCart)
    (CallFunction|MovingPopcornActor)))

(event Collision|EventActorBeginOverlap
  (params (OtherActor :type Actor%20Object%20Reference))
  (Utilities|Casting|CastToFirstPersonProjectile OtherActor)
  (Variables|Default|SetCurrentHealth (- (Variables|Default|GetCurrentHealth) 1e+01))
  (if (<= (Variables|Default|GetCurrentHealth) 0.0)
    (Actor|DestroyActor)))

(fn ConstructionScript)