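; Shootable target that keeps hopping around the level and explodes when hit by a FirstPersonProjectile.
; On BeginPlay and each component hit, LaunchActor impulses it along a suggested high-arc toss toward a random point in the first SpawnVolume found.
; A failed cast to BP_HoffmannMehatGameMode flags free play, so overlaps report hits and kills to FreePlayGameMode; otherwise that mode also gets score.
; Older interpolated movement, look-at and LaunchCharacter logic is left disconnected.
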(event OnComponentHit(TheFirstActor)
  (params (HitComponent :type Primitive%20Component%20Object%20Reference) (OtherActor :type Actor%20Object%20Reference) (OtherComp :type Primitive%20Component%20Object%20Reference) (NormalImpulse :type Vector :default "0, 0, 0") (Hit :type Hit%20Result%20Structure%20%28by%20ref%29))
  (CallFunction|LaunchActor))

(event Collision|EventActorBeginOverlap
  (params (OtherActor :type Actor%20Object%20Reference))
  (if (Variables|Default|GetisFreePlay)
    (bind _asfirst_person_projectile (Utilities|Casting|CastToFirstPersonProjectile OtherActor))
    (bind _asfree_play_game_mode (Utilities|Casting|CastToFreePlayGameMode (Game|GetGameMode)))
    (Default|TargetHit _asfree_play_game_mode)
    (Default|AddKill _asfree_play_game_mode)
    (Effects|SpawnEmitteratLocation "/Game/Blueprints/ExplosionParticle.ExplosionParticle" (Transformation|GetActorLocation) (Transformation|GetActorRotation))
    (Actor|DestroyActor _asfirst_person_projectile)
    (Actor|DestroyActor)
    (else
      (bind _asfirst_person_projectile_2 (Utilities|Casting|CastToFirstPersonProjectile OtherActor))
      (Utilities|FlowControl|Sequence
        (:then_0
          ;[1 1 1] Update Player Score
          (bind _asbp_hoffmann_mehat_game_mode (Utilities|Casting|CastToBP_HoffmannMehatGameMode (Game|GetGameMode)))
          (Default|TargetScore _asbp_hoffmann_mehat_game_mode (Variables|Default|Gettargetscore)))
        (:then_1
          ;[1 1 1] Spawn Explostion Particles
          (Effects|SpawnEmitteratLocation "/Game/Blueprints/ExplosionParticle.ExplosionParticle" (Transformation|GetActorLocation) (Transformation|GetActorRotation)))
        (:then_2
          (bind _asbp_hoffmann_mehat_game_mode_2 (Utilities|Casting|CastToBP_HoffmannMehatGameMode (Game|GetGameMode)))
          ;[1 1 1] This adds one to the HitTheTarget counter varaiable in HoffmannMehatGameMode
          (Default|TargetHit _asbp_hoffmann_mehat_game_mode_2 1))
        (:then_3
          ;[1 1 1] Destroy Actor
          (Default|AddKill _asbp_hoffmann_mehat_game_mode)
          (Actor|DestroyActor _asfirst_person_projectile_2)
          (Actor|DestroyActor))))))

(event EventBeginPlay
  (bind _outactors (Actor|GetAllActorsOfClass "/Script/HoffmannMehat.SpawnVolume"))
  (Variables|Default|SetSpawnVolume (Utilities|Array|Get(acopy) _outactors))
  (CallFunction|LaunchActor)
  (bind _asbp_hoffmann_mehat_game_mode (Utilities|Casting|CastToBP_HoffmannMehatGameMode (Game|GetGameMode))
    (:then
      (Variables|/Game/FirstPersonCPP/Blueprints/BP_HoffmannMehatGameMode.BP_HoffmannMehatGameMode_C|SetTimeBeginInterval _asbp_hoffmann_mehat_game_mode (Math|DateTime|Now)))
    (:CastFailed
      (Variables|Default|SetisFreePlay true))))

(fn ConstructionScript)

(fn CheckLocation
  (params (actLocation :type Vector))
  (return (<= (- (.Z (Math|Vector|BreakVector actLocation)) 2.1e+02) 1e+02)))

(fn LaunchActor
  (bind _returnvalue (Class|SpawnVolume|GetRandomPointinVolume (Variables|Default|GetSpawnVolume)))
  (bind _tossvelocity (Class|GameplayStatics|BlueprintSuggestProjectileVelocity (Transformation|GetActorLocation) _returnvalue 1e+03 0.0 "DoNotTrace" 0.0 true false))
  (Physics|AddImpulse (Variables|Default|GetTheFirstActor) _tossvelocity "None" true))