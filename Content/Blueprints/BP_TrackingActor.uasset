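; BP_TrackingActor is a flying shooting target that roams inside a SpawnVolume while turning to face the player.
; BeginPlay finds the first SpawnVolume and picks a random point in it as the flight target.
; Tick rotates toward the player and moves at constant speed to that point, choosing a new one on arrival.
; Overlap by a FirstPersonProjectile reports its score to the game mode, spawns an explosion and destroys it.
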(event EventBeginPlay
  ;[1 1 1] Sets the Original Flight Target
  (bind _outactors (Actor|GetAllActorsOfClass "/Script/HoffmannMehat.SpawnVolume"))
  (bind _output_get (Variables|Default|SetSpawnVolume (Utilities|Array|Get(acopy) _outactors)))
  (bind _returnvalue (Class|SpawnVolume|GetRandomPointinVolume _output_get))
  (Variables|Default|SetFlightTarget _returnvalue))

(event Collision|EventActorBeginOverlap
  (params (OtherActor :type Actor%20Object%20Reference))
  (Utilities|Casting|CastToFirstPersonProjectile OtherActor)
  (Utilities|FlowControl|Sequence
    (:then_0
      ;[1 1 1] Update Player Score
      (bind _asbp_hoffmann_mehat_game_mode (Utilities|Casting|CastToBP_HoffmannMehatGameMode (Game|GetGameMode)))
      (Default|TargetScore _asbp_hoffmann_mehat_game_mode (Variables|Default|Gettargetscore)))
    (:then_1
      ;[1 1 1] Spawn Explostion Particles
      (Effects|SpawnEmitteratLocation "/Game/Blueprints/ExplosionParticle.ExplosionParticle" (Transformation|GetActorLocation) (Transformation|GetActorRotation)))
    (:then_2
      ;[1 1 1] Destroy Actor
      (Actor|DestroyActor))))

(event EventTick
  (params (DeltaSeconds :type Float%20%28single-precision%29))
  (bind _returnvalue (Transformation|GetActorLocation))
  ;[1 1 1] Orient Target Towards Player
  (Transformation|SetActorRotation (Math|Rotator|FindLookatRotation (Transformation|GetActorLocation) (Transformation|GetActorLocation (Game|GetPlayerCharacter 0))))
  ;[1 1 1] Responsible For Randomly Moving the Actor
  (bind _issame (CallFunction|CheckLocation _returnvalue (Variables|Default|GetFlightTarget)))
  (if _issame
    (bind _returnvalue_2 (Class|SpawnVolume|GetRandomPointinVolume (Variables|Default|GetSpawnVolume)))
    (bind _output_get (Variables|Default|SetFlightTarget _returnvalue_2))
    (Transformation|SetActorLocation (Math|Interpolation|VInterptoConstant _returnvalue _output_get DeltaSeconds 1e+03) false false)
    (else
      (Transformation|SetActorLocation (Math|Interpolation|VInterptoConstant _returnvalue (Variables|Default|GetFlightTarget) DeltaSeconds 1e+03) false false))))

(fn ConstructionScript)

(fn CheckLocation
  (params (ActorLocation :type Vector) (TargetPoint :type Vector))
  (return (Math|Vector|Equal(Vector) ActorLocation TargetPoint 0.1)))