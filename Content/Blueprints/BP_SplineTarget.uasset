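; BP_SplineTarget is a shootable target that rides along a level spline while turning to face the player.
; The construction script picks a random LevelSpline, start offset and travel time.
; On BeginPlay, the CartMover timeline uses these to drive the target by distance along the spline.
; Overlap with a FirstPersonProjectile passes its score to the game mode, spawns explosion particles and destroys the target.
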(event Custom|MoveCart
  ;[1 1 1] Spline Target Isn't moving
  (Components|Timeline|SetPlayRate (Variables|Default|GetCartMover) (/ 1.0 (Variables|Default|GetCartSpeed)))
  (Components|Timeline|SetNewTime (Variables|Default|GetCartMover) (Variables|Default|GetCartStartOffset))
  (bind _alpha (Timeline|CartMover Play)
    (:Update
      (Variables|Default|SetAlpha _alpha)
      (Transformation|SetActorLocationAndRotation (Spline|GetLocationatDistanceAlongSpline (Variables|/Game/Blueprints/LevelSpline.LevelSpline_C|GetSpline (Variables|Default|GetTrackRef)) (Math|Float|Lerp 0.0 (Spline|GetSplineLength (Variables|/Game/Blueprints/LevelSpline.LevelSpline_C|GetSpline (Variables|Default|GetTrackRef))) (Variables|Default|GetAlpha)) "World") (Math|Rotator|FindLookatRotation (Transformation|GetActorLocation) (Transformation|GetActorLocation (Game|GetPlayerCharacter 0)))))))

(event EventBeginPlay
  (CallFunction|MoveCart))

(event Collision|EventActorBeginOverlap
  (params (OtherActor :type Actor%20Object%20Reference))
  (Utilities|Casting|CastToFirstPersonProjectile OtherActor)
  (Utilities|FlowControl|Sequence
    (:then_0
      ;[1 1 1] Update Player Score
      (bind _asbp_hoffmann_mehat_game_mode (Utilities|Casting|CastToBP_HoffmannMehatGameMode (Game|GetGameMode)))
      (Default|TargetScore _asbp_hoffmann_mehat_game_mode (Variables|Default|Gettargetscore)))
    (:then_1
      ;[1 1 1] Spawn Explostion Particles
      (Effects|SpawnEmitteratLocation "/Game/Blueprints/ExplosionParticle.ExplosionParticle" (Transformation|GetActorLocation) (Transformation|GetActorRotation)))
    (:then_2
      ;[1 1 1] Destroy Actor
      (Actor|DestroyActor))))

(fn ConstructionScript
  (bind _outactors (Actor|GetAllActorsOfClass "/Game/Blueprints/LevelSpline.LevelSpline_C"))
  (Variables|Default|SetTrackRef (Utilities|Array|Get(acopy) _outactors (Math|Random|RandomInteger (Utilities|Array|Length _outactors))))
  (Variables|Default|SetCartStartOffset (Math|Random|RandomFloat))
  (Variables|Default|SetCartSpeed (Math|Random|RandomFloatinRange 1e+01 3e+01)))

(fn CheckLocation
  (params (ActorLocation :type Vector) (TargetPoint :type Vector))
  (return (Math|Vector|Equal(Vector) ActorLocation TargetPoint 0.1)))