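; Shootable target actor that turns to face the player every tick and explodes, destroying itself and the projectile, when overlapped by a FirstPersonProjectile.
; Under BP_HoffmannMehatGameMode, a hit also reports score and hit to the game mode and updates its time between kills, with the interval timer started on BeginPlay.
; If that game mode cast fails on BeginPlay, the target switches to free play and skips all scoring and timing.
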(event EventBeginPlay
  (bind _asbp_hoffmann_mehat_game_mode (Utilities|Casting|CastToBP_HoffmannMehatGameMode (Game|GetGameMode))
    (:then
      (Variables|/Game/FirstPersonCPP/Blueprints/BP_HoffmannMehatGameMode.BP_HoffmannMehatGameMode_C|SetTimeBeginInterval _asbp_hoffmann_mehat_game_mode (Math|DateTime|Now)))
    (:CastFailed
      (Variables|Default|SetisFreePlay true))))

(event Collision|EventActorBeginOverlap
  (params (OtherActor :type Actor%20Object%20Reference))
  (if (Variables|Default|GetisFreePlay)
    (bind _asfirst_person_projectile (Utilities|Casting|CastToFirstPersonProjectile OtherActor))
    (Effects|SpawnEmitteratLocation "/Game/Blueprints/ExplosionParticle.ExplosionParticle" (Transformation|GetActorLocation) (Transformation|GetActorRotation))
    (Actor|DestroyActor _asfirst_person_projectile)
    (Actor|DestroyActor)
    (else
      (bind _asfirst_person_projectile_2 (Utilities|Casting|CastToFirstPersonProjectile OtherActor))
      (Utilities|FlowControl|Sequence
        (:then_0
          ;[1 1 1] Update Player Score
          (bind _asbp_hoffmann_mehat_game_mode (Utilities|Casting|CastToBP_HoffmannMehatGameMode (Game|GetGameMode)))
          (Default|TargetScore _asbp_hoffmann_mehat_game_mode (Variables|Default|Gettargetscore)))
        (:then_1
          (bind _asbp_hoffmann_mehat_game_mode_2 (Utilities|Casting|CastToBP_HoffmannMehatGameMode (Game|GetGameMode)))
          (Default|TargetHit _asbp_hoffmann_mehat_game_mode_2 (Variables|Default|GetHitTarget)))
        (:then_2
          ;[1 1 1] Spawn Explostion Particles
          (Effects|SpawnEmitteratLocation "/Game/Blueprints/ExplosionParticle.ExplosionParticle" (Transformation|GetActorLocation) (Transformation|GetActorRotation)))
        (:then_3
          ;[1 1 1] Calculating TimeBtwnKill + Destroying Actor
          (bind _asbp_hoffmann_mehat_game_mode_3 (Utilities|Casting|CastToBP_HoffmannMehatGameMode (Game|GetGameMode)))
          (Variables|/Game/FirstPersonCPP/Blueprints/BP_HoffmannMehatGameMode.BP_HoffmannMehatGameMode_C|SetTimeEndInterval _asbp_hoffmann_mehat_game_mode_3 (Math|DateTime|Now))
          (Variables|/Game/FirstPersonCPP/Blueprints/BP_HoffmannMehatGameMode.BP_HoffmannMehatGameMode_C|SetTimeBtwnKill _asbp_hoffmann_mehat_game_mode_3 (- (Variables|/Game/FirstPersonCPP/Blueprints/BP_HoffmannMehatGameMode.BP_HoffmannMehatGameMode_C|GetTimeEndInterval _asbp_hoffmann_mehat_game_mode_3) (Variables|/Game/FirstPersonCPP/Blueprints/BP_HoffmannMehatGameMode.BP_HoffmannMehatGameMode_C|GetTimeBeginInterval _asbp_hoffmann_mehat_game_mode_3)))
          (Variables|/Game/FirstPersonCPP/Blueprints/BP_HoffmannMehatGameMode.BP_HoffmannMehatGameMode_C|SetTimeBeginInterval _asbp_hoffmann_mehat_game_mode_3 (Math|DateTime|Now))
          (Actor|DestroyActor _asfirst_person_projectile_2)
          (Actor|DestroyActor))))))

(event EventTick
  (params (DeltaSeconds :type Float%20%28single-precision%29))
  ;[1 1 1] Orient Target Towards Player
  (Transformation|SetActorRotation (Math|Rotator|FindLookatRotation (Transformation|GetActorLocation) (Transformation|GetActorLocation (Game|GetPlayerCharacter 0)))))

(fn ConstructionScript)